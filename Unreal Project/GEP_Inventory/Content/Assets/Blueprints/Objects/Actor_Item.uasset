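; Actor_Item is a world pickup that gives its Item to the player on contact.
; The construction script sets the static mesh and its first material from the Item's data when the Item is valid.
; On overlap with an Actor_Player, it passes the Item to that player's AddItem and then destroys itself.
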(event `self.ReceiveActorBeginOverlap`
  (params (OtherActor :type "Actor Object Reference"))
  (bind _asactor_player (cast `/Game/Assets/Blueprints/Player/Actor_Player` OtherActor))
  (`/Game/Assets/Blueprints/Player/Actor_Player.AddItem` _asactor_player (`self.Item`))
  (`self.K2_DestroyActor`))

(fn `UserConstructionScript`
  (bind _staticmesh (`self.StaticMesh`))
  (bind _item (`self.Item`)
    (:`then`
      (`StaticMeshComponent.SetStaticMesh` _staticmesh (`/Game/Assets/DataAssets/Data_Item.item_mesh` _item))
      (`PrimitiveComponent.SetMaterial` _staticmesh 0 (`/Game/Assets/DataAssets/Data_Item.item_material` _item)))
    (:`else`)))