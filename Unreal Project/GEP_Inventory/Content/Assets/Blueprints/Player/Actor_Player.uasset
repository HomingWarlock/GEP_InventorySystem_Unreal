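; Player actor with first-person movement, a crosshair HUD and a simple item inventory.
; Axis inputs drive look and movement unless MovementLocked, which the inventory toggle sets while swapping crosshair, inventory widget, input mode and cursor.
; Pickup line-traces from the camera, adds a hit Actor_Item's item to the Inventory array and destroys the actor.
; Adding or removing items rebuilds the inventory widget's entries from that array.
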(event `InputAxis|Rotate_Left_Right`
  (params (AxisValue :type "Float (single-precision)"))
  ;[0 0 1 1 30] Movement
  ;;[1 1 1] Mouse Rotation
  (if (not (`self.movement_locked`))
    (`self.AddControllerYawInput` AxisValue)))

(event `InputAxis|Look_Up_Down`
  (params (AxisValue :type "Float (single-precision)"))
  ;[0 0 1 1 30] Movement
  ;;[1 1 1] Mouse Rotation
  (if (not (`self.movement_locked`))
    (`self.AddControllerPitchInput` AxisValue)))

(event `InputAxis|Forward_Backward`
  (params (AxisValue :type "Float (single-precision)"))
  ;[0 0 1 1 30] Movement
  ;;[1 1 1] Forward and Back Movement
  (if (not (`self.movement_locked`))
    (`self.AddMovementInput` (`self.GetActorForwardVector`) AxisValue)))

(event `InputAxis|Strafe_Left_Right`
  (params (AxisValue :type "Float (single-precision)"))
  ;[0 0 1 1 30] Movement
  ;;[1 1 1] Strafe Left and Right
  (if (not (`self.movement_locked`))
    (`self.AddMovementInput` (`self.GetActorRightVector`) AxisValue)))

(event `self.ReceiveBeginPlay`
  (bind _returnvalue (`GameplayStatics.GetPlayerController` 0))
  ;[0 1 0 1 30] Create GUI
  (bind _returnvalue_2 (`|CreateWidget` "/Game/Assets/GUI/Crosshair.Crosshair_C" _returnvalue))
  (bind _output_get (set `self.CrossHairWidget` _returnvalue_2))
  (`UserWidget.AddToViewport` _output_get 0)
  (`Widget.SetVisibility` _output_get "Visible")
  (bind _returnvalue_3 (`|CreateWidget` "/Game/Assets/GUI/InventoryUI.InventoryUI_C" _returnvalue))
  (set `self.InventoryWidget` _returnvalue_3))

(event `InputAction|Inventory_Open_Close`
  (params (Key :type "Key Structure"))
  (bind _returnvalue (`GameplayStatics.GetPlayerController` 0))
  (bind _inventorywidget (`self.InventoryWidget`))
  (bind _crosshairwidget (`self.CrossHairWidget`))
  ;[1 1 0 1 30] Toggle Inventory
  (:`Pressed`
    (`/Engine/EditorBlueprintResources/StandardMacros.FlipFlop`
      (:`A`
        (set `self.movement_locked` true)
        (`UserWidget.AddToViewport` _inventorywidget 0)
        (`Widget.SetVisibility` _inventorywidget "Visible")
        (`Widget.SetVisibility` _crosshairwidget "Hidden")
        (`WidgetBlueprintLibrary.SetInputMode_GameAndUIEx` _returnvalue null)
        (set `PlayerController.bShowMouseCursor` true _returnvalue))
      (:`B`
        (set `self.movement_locked` false)
        (`Widget.SetVisibility` _inventorywidget "Hidden")
        (`UserWidget.AddToViewport` _crosshairwidget 0)
        (`Widget.SetVisibility` _crosshairwidget "Visible")
        (`WidgetBlueprintLibrary.SetInputMode_GameOnly` _returnvalue)
        (set `PlayerController.bShowMouseCursor` false _returnvalue)))))

(event `InputAction|Pickup_Item`
  (params (Key :type "Key Structure"))
  (bind _fpcam (`self.FPCam`))
  (bind _returnvalue (`SceneComponent.K2_GetComponentLocation` _fpcam))
  ;[1 1 1 1 30] Pickup Item
  (:`Pressed`
    (bind (_outhit _returnvalue_2) (`KismetSystemLibrary.LineTraceSingle` _returnvalue (+ _returnvalue (* (`SceneComponent.GetForwardVector` _fpcam) 250.0)) "TraceTypeQuery1"))
    (if _returnvalue_2
      (bind _asactor_item (cast `/Game/Assets/Blueprints/Objects/Actor_Item` (`.HitActor` (`GameplayStatics.BreakHitResult` _outhit))))
      (`self.AddItem` (`/Game/Assets/Blueprints/Objects/Actor_Item.Item` _asactor_item))
      (`self.K2_DestroyActor` _asactor_item))))

(fn `AddItem`
  (params (NewItem :type "/Game/Assets/DataAssets/Data_Item Object Reference (by ref)"))
  (`KismetArrayLibrary.Array_Add` (`self.Inventory`) NewItem)
  (`self.CreateInventory`))

(fn `CreateInventory`
  (`PanelWidget.ClearChildren` (`/Game/Assets/GUI/InventoryUI.Content` (`self.InventoryWidget`)))
  (for (_array_element _array_index) (`self.Inventory`)
    (`/Game/Assets/GUI/InventoryUI.DrawNewItem` (`self.InventoryWidget`) _array_element _array_index)))

(fn `RemoveItem`
  (params (IndexToRemove :type Integer))
  (`KismetArrayLibrary.Array_Remove` (`self.Inventory`) IndexToRemove)
  (`self.CreateInventory`))

(fn `UserConstructionScript`)